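; BP_Marine is a player pawn that moves along fixed world X and Y axes and aims independently of movement.
; Each tick, UpdatePlayerAim turns mouse velocity into a yaw angle and smoothly interpolates control rotation toward it, ignoring motion within a deadzone.
; A matching gamepad thumbstick aim branch exists but is disconnected, so only mouse aiming runs.
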(event EventBeginPlay)

(event Collision|EventActorBeginOverlap
  (params (OtherActor :type Actor%20Object%20Reference)))

(event EventTick
  (params (DeltaSeconds :type Float%20%28single-precision%29))
  (CallFunction|UpdatePlayerAim))

(event Input|AxisEvents|InputAxisMoveForeward
  (params (AxisValue :type Float%20%28single-precision%29))
  (Pawn|Input|AddMovementInput "1.000000, 0, 0" AxisValue false))

(event Input|AxisEvents|InputAxisMoveRight
  (params (AxisValue :type Float%20%28single-precision%29))
  (Pawn|Input|AddMovementInput "0.000000,1.000000, 0" AxisValue false))

(fn ConstructionScript)

(fn UpdatePlayerAim
  (bind _returnvalue (Game|GetPlayerController 0))
  (bind _mousevelocity (CallFunction|GetMouseVelocity))
  ;[1 1 1] MouseRotation
  (if (CallFunction|IsMouseAboveDeadzone)
    (Pawn|SetControlRotation _returnvalue (Math|Interpolation|RInterpTo (Pawn|GetControlRotation _returnvalue :!class /Script/Engine.Controller) (Math|Rotator|MakeRotator 0.0 0.0 (Class|KismetMathLibrary|DegAtan2 (.x _mousevelocity) (.y _mousevelocity))) (Utilities|Time|GetWorldDeltaSeconds) (Variables|Setup|GetMouseRotationSmoothingStrength)))))

(fn IsThumbstickAboveDeadzone
  (return (> (Math|Vector2D|Vector2DLength (Math|Vector2D|MakeVector2D (Input|AxisValues|GetThumbsticAimUp) (Input|AxisValues|GetThumbsticAimRight))) (Variables|Setup|GetThumbstickDeadzone))))

(fn GetMouseVelocity
  (bind _returnvalue (Game|GetPlayerController 0))
  (bind (_deltax _deltay) (Class|PlayerController|GetInputMouseDelta _returnvalue))
  (return (/ (Math|Vector2D|MakeVector2D _deltax _deltay) (Utilities|Time|GetWorldDeltaSeconds))))

(fn IsMouseAboveDeadzone
  (return (> (Math|Vector2D|Vector2DLength (CallFunction|GetMouseVelocity)) (Variables|Setup|GetMouseDeadzone))))